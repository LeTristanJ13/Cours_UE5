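; BP_Porte is a door that slides between two positions when it receives an Activate or Disable event.
; Both events call the same OpenDoor function, so each acts as a toggle rather than setting an explicit open or closed state.
; OpenDoor checks the Door component's relative Y location and instantly snaps it to either the origin or a sideways offset, with no animation or sweep.
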(event `/Game/Blueprint/BPI_InterrupteurControlable.Disable`
  (`self.OpenDoor`))

(event `/Game/Blueprint/BPI_InterrupteurControlable.Activate`
  (`self.OpenDoor`))

(fn `OpenDoor`
  (bind (_relativelocation_x _relativelocation_y) (`KismetMathLibrary.BreakVector` (`SceneComponent.RelativeLocation` (`self.Door`))))
  (if (> _relativelocation_y 0.0)
    (`SceneComponent.K2_SetRelativeLocation` (`self.Door`) (0.0 0.0 0.0) false false)
    (else
      (`SceneComponent.K2_SetRelativeLocation` (`self.Door`) (0.0 100.0 0.0) false false))))

(fn `UserConstructionScript`)