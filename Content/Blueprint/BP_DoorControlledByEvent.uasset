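; BP_DoorControlledByEvent is a door that slides along its local Y axis when an external event fires.
; On BeginPlay it binds Activate to EventLauncher's activation event for controllables.
; Activate instantly offsets the door if its Y is not positive; otherwise it adds zero, so an open door stays open.
; A separate OpenDoor function, uncalled here, toggles between closed and open using absolute relative locations.
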(event `self.ReceiveBeginPlay`
  (add `/Game/Blueprint/BP_InterrupteurEventLauncher.ActivateControlables` (`self.EventLauncher`) (delegate `Activate`)))

(event `Activate`
  (bind _door (`self.Door`))
  (bind (_relativelocation_x _relativelocation_y) (`KismetMathLibrary.BreakVector` (`SceneComponent.RelativeLocation` _door)))
  (if (> _relativelocation_y 0.0)
    (`SceneComponent.K2_AddRelativeLocation` _door (0.0 0.0 0.0) false false)
    (else
      (`SceneComponent.K2_AddRelativeLocation` _door (0.0 150.0 0.0) false false))))

(fn `OpenDoor`
  (bind (_relativelocation_x _relativelocation_y) (`KismetMathLibrary.BreakVector` (`SceneComponent.RelativeLocation` (`self.Door`))))
  (if (> _relativelocation_y 0.0)
    (`SceneComponent.K2_SetRelativeLocation` (`self.Door`) (0.0 0.0 0.0) false false)
    (else
      (`SceneComponent.K2_SetRelativeLocation` (`self.Door`) (0.0 100.0 0.0) false false))))

(fn `UserConstructionScript`)