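; Door Blueprint that two switch actors toggle through event dispatchers bound on BeginPlay.
; OpenPorte requires BP_ThirdPersonGameMode, then loops over BPControllable actors implementing BPI_Exo.
; Each matching actor snaps the door yaw between 0 and 90 degrees, so the toggle repeats per element.
; That actor receives ActivableMessage when yaw resets to 0 or DisableMessage when set to 90, with a debug print.
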(event `self.ReceiveBeginPlay`
  (add `/Game/Blueprint/Exercice/BP_Interrupteur_Second1.EventOpenDoor1_2` (`self.BP_InterrupteurSecond1`) (delegate `OpenDoor`))
  (add `/Game/Blueprint/Exercice/BP_Interrupteur_Second3.EventOpenDoors1_3` (`self.BP_InterrupteurSecond3`) (delegate `OpenDoor`)))

(event `OpenDoor`
  (`self.OpenPorte`))

(fn `OpenPorte`
  (bind (_relativerotation_roll _relativerotation_pitch _relativerotation_yaw) (`KismetMathLibrary.BreakRotator` (`SceneComponent.RelativeRotation` (`self.Door`))))
  (cast `/Game/ThirdPerson/Blueprints/BP_ThirdPersonGameMode` (`GameplayStatics.GetGameMode`))
  (for _array_element (`self.BP_Controllable`)
    (if (`KismetSystemLibrary.DoesImplementInterface` _array_element "/Game/Blueprint/Exercice/BPI_Exo.BPI_Exo_C")
      (if (> _relativerotation_yaw 0.0)
        (`SceneComponent.K2_SetRelativeRotation` :`self` (`self.Door`))
        (message `/Game/Blueprint/Exercice/BPI_Exo.Activable` _array_element)
        (`KismetSystemLibrary.PrintString` "Je m'active et je fais +1")
        (else
          (`SceneComponent.K2_SetRelativeRotation` (`self.Door`) (struct :`Yaw` 90.0) false false)
          (message `/Game/Blueprint/Exercice/BPI_Exo.Disable` _array_element)
          (`KismetSystemLibrary.PrintString` "Je m'active et je fais -1"))))))

(fn `UserConstructionScript`)