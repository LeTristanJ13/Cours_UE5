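; BP_Lampadaire is an exercise street lamp whose point light is toggled by a counter driven from outside events.
; Activable increments Compteur and Disable decrements it, then both call LightOn.
; LightOn prints the count in French and shows the PointLight only when the count is exactly zero, hiding it for any other value.
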(event `/Game/Blueprint/Exercice/BPI_Exo.Activable`
  (set `self.Compteur` (+ 1 (`self.Compteur`)))
  (`self.LightOn`))

(event `/Game/Blueprint/Exercice/BPI_Exo.Disable`
  (set `self.Compteur` (- (`self.Compteur`) 1))
  (`self.LightOn`))

(fn `LightOn`
  (bind _pointlight (`self.PointLight`))
  (bind _compteur (`self.Compteur`))
  (`KismetSystemLibrary.PrintString` (`KismetStringLibrary.Concat_StrStr` "Le compteur est égal a :" (`KismetStringLibrary.Conv_IntToString` _compteur)))
  (if (== _compteur 0)
    (`SceneComponent.SetVisibility` _pointlight true false)
    (else
      (`SceneComponent.SetVisibility` _pointlight false false))))

(fn `UserConstructionScript`)