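; BP_Porte is a door actor that toggles open and closed in response to two switch Blueprints.
; On BeginPlay it binds its OpenDoor event to the dispatchers of its two referenced switches, so either one can trigger it.
; OpenPorte checks the Door component's relative yaw and snaps it between closed and a quarter-turn open, with no interpolation.
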(event `self.ReceiveBeginPlay`
  (add `/Game/Blueprint/Exercice/BP_Interrupteur_Second1.EventOpenDoor1_2` (`self.BP_InterrupteurSecond1`) (delegate `OpenDoor`))
  (add `/Game/Blueprint/Exercice/BP_Interrupteur_Second3.EventOpenDoors1_3` (`self.BP_InterrupteurSecond3`) (delegate `OpenDoor`)))

(event `OpenDoor`
  (`self.OpenPorte`))

(fn `OpenPorte`
  (bind _door (`self.Door`))
  (bind (_relativerotation_roll _relativerotation_pitch _relativerotation_yaw) (`KismetMathLibrary.BreakRotator` (`SceneComponent.RelativeRotation` _door)))
  (if (> _relativerotation_yaw 0.0)
    (`SceneComponent.K2_SetRelativeRotation` _door (struct) false false)
    (else
      (`SceneComponent.K2_SetRelativeRotation` _door (struct :`Yaw` 90.0) false false))))

(fn `UserConstructionScript`)